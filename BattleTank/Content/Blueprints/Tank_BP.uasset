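; Tank pawn Blueprint that wires player input to the tank's aiming and movement components.
; On BeginPlay it passes the barrel and turret to TankAiming and both tracks to TankMovement.
; Axis inputs drive each track's throttle directly or go through TankMovement as forward and turn intent, while Fire calls TankAiming.
; Aim axes rotate a yaw gimbal and spring arm separately, scaled by delta time.
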(event `self.ReceiveBeginPlay`
  (`TankAimingComponent.Initialise` (`self.TankAiming`) (`self.Barrel`) (`self.Turret`))
  (`TankMovementComponent.Initialise` (`self.TankMovement`) (`self.Left Track`) (`self.Right Track`)))

(event `InputAxis|Left Track Throttle`
  (params (AxisValue :type "Float (single-precision)"))
  (`TankTrack.SetThrottle` (`self.Left Track`) AxisValue))

(event `InputAxis|AimYaw`
  (params (AxisValue :type "Float (single-precision)"))
  (`SceneComponent.K2_AddLocalRotation` (`self.Yaw Gimble`) (`KismetMathLibrary.MakeRotator` 0.0 0.0 (* AxisValue (`GameplayStatics.GetWorldDeltaSeconds`) 100.0)) false false))

(event `InputAxis|Right Track Throttle`
  (params (AxisValue :type "Float (single-precision)"))
  (`TankTrack.SetThrottle` (`self.Right Track`) AxisValue))

(event `InputAxis|AimElevation`
  (params (AxisValue :type "Float (single-precision)"))
  (`SceneComponent.K2_AddLocalRotation` (`self.SpringArm`) (`KismetMathLibrary.MakeRotator` 0.0 (* AxisValue (`GameplayStatics.GetWorldDeltaSeconds`) 100.0)) false false))

(event `InputAxis|Tank Forward Movement`
  (params (AxisValue :type "Float (single-precision)"))
  (`TankMovementComponent.IntendedForwardMove` (`self.TankMovement`) AxisValue))

(event `InputAxis|Tank Right Movement`
  (params (AxisValue :type "Float (single-precision)"))
  (`TankMovementComponent.IntendedTurnRight` (`self.TankMovement`) AxisValue))

(event `InputAction|Fire`
  (params (Key :type "Key Structure" :default "AnyKey"))
  (:`Pressed`
    (`TankAimingComponent.Fire` (`self.TankAiming`))))

(fn `UserConstructionScript`)